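; Player grappling hook Blueprint that attaches to a surface while the right mouse button is held.
; Pressing sphere-traces from CableMark to an endpoint that multiplies, rather than offsets, its location by scaled camera forward, storing any hit as HookPoint.
; While connected, Tick feeds CharacterMovement a force along the hook-to-player axis, scaled by offset dot velocity, plus constant camera-forward thrust.
; Releasing the button disconnects the grapple.
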(event `Key|RightMouseButton`
  (params (Key :type "Key Structure"))
  (bind _returnvalue (`SceneComponent.K2_GetComponentLocation` (`self.CableMark`)))
  (:`Pressed`
    (bind (_outhit _returnvalue_2) (`KismetSystemLibrary.SphereTraceSingle` _returnvalue (* _returnvalue (* (`self.GetActorForwardVector` (`GameplayStatics.GetPlayerCameraManager` 0)) (`self.Hook Distance`))) 15.0 "TraceTypeQuery1"))
    (if _returnvalue_2
      (set `self.Hook Point` (`.ImpactPoint` (`GameplayStatics.BreakHitResult` _outhit)))
      (set `self.Grapple Connected` true)))
  (:`Released`
    (set `self.Grapple Connected` false)))

(event `self.ReceiveTick`
  (params (DeltaSeconds :type "Float (single-precision)"))
  (bind _returnvalue (- (`self.K2_GetActorLocation`) (`self.Hook Point`)))
  (if (`self.Grapple Connected`)
    (`CharacterMovementComponent.AddForce` (`self.Character movement`) (* (`KismetMathLibrary.Normal` _returnvalue) (`KismetMathLibrary.Dot_VectorVector` _returnvalue (`self.GetVelocity`))))
    (`CharacterMovementComponent.AddForce` (`self.Character movement`) (* (`self.GetActorForwardVector` (`GameplayStatics.GetPlayerCameraManager` 0)) 50000.0))))

(fn `UserConstructionScript`)
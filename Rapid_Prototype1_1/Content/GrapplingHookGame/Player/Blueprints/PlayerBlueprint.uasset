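; Player character for a grappling-hook shooter, with movement, camera look, bullet firing and grappling.
; Grapple sphere-traces along the camera forward; on a hit it spawns a hook point actor and attaches the visible cable to it.
; While connected, Tick applies a velocity-dependent force along the rope axis, plus a camera-forward push for a steerable swing.
; On destruction it releases the grapple and, after a delay, opens a level to respawn.
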(event `InputAction|Jump`
  (params (Key :type "Key Structure"))
  ;[1 1 1] Movement inputs
  (:`Pressed`
    (`self.Jump`))
  (:`Released`
    (`self.StopJumping`)))

(event `InputAxis|MoveForward`
  (params (AxisValue :type "Float (single-precision)"))
  ;[1 1 1] Movement inputs
  (`self.AddMovementInput` (`SceneComponent.GetForwardVector` (`self.Camera`)) AxisValue))

(event `InputAxis|MoveRight`
  (params (AxisValue :type "Float (single-precision)"))
  ;[1 1 1] Movement inputs
  (`self.AddMovementInput` (`SceneComponent.GetRightVector` (`self.Camera`)) AxisValue))

(event `InputAction|Shoot`
  (params (Key :type "Key Structure"))
  ;[1 1 1] Create bullet
  (:`Pressed`
    (set `self.isLeftDown` true)
    (`GameplayStatics.PlaySoundAtLocation` "/Game/GrapplingHookGame/Player/Audio/369528__johandeecke__short-gunshot.369528__johandeecke__short-gunshot" (0.0 0.0 0.0) (struct) 1.0 1.0 0.0 null null null)
    (`self.SpawnBullet`))
  (:`Released`
    (set `self.isLeftDown` false)))

(event `self.ReceiveTick`
  (params (DeltaSeconds :type "Float (single-precision)"))
  (bind _returnvalue (- (`self.K2_GetActorLocation`) (`self.Hook Point`)))
  ;[1 1 1] Update
  (if (`self.Grapple Connected`)
    (`CharacterMovementComponent.AddForce` (`self.CharacterMovement`) (* (* (`KismetMathLibrary.Normal` _returnvalue) (`KismetMathLibrary.Dot_VectorVector` _returnvalue (`self.GetVelocity`))) -10.0))
    (`CharacterMovementComponent.AddForce` (`self.CharacterMovement`) (* (`self.GetActorForwardVector` (`GameplayStatics.GetPlayerCameraManager` 0)) 50000.0))))

(event `InputAxis|Turn`
  (params (AxisValue :type "Float (single-precision)"))
  ;[1 1 1] Camera rotation
  (`self.AddControllerYawInput` AxisValue))

(event `InputAxis|LookUp`
  (params (AxisValue :type "Float (single-precision)"))
  ;[1 1 1] Camera rotation
  (`SceneComponent.K2_AddLocalRotation` (`self.Camera`) (`KismetMathLibrary.MakeRotator` 0.0 AxisValue) false false))

(event `InputAction|Grapple`
  (params (Key :type "Key Structure"))
  (bind _returnvalue (`SceneComponent.K2_GetComponentLocation` (`self.CableMark`)))
  ;[1 1 1] Grapple inputs
  (:`Pressed`
    (set `self.isRightDown` true)
    (`GameplayStatics.PlaySoundAtLocation` "/Game/GrapplingHookGame/Player/Audio/366248__kfatehi__hook.366248__kfatehi__hook" (0.0 0.0 0.0) (struct) 1.0 1.0 0.0 null null null)
    (bind (_outhit _returnvalue_2) (`KismetSystemLibrary.SphereTraceSingle` _returnvalue (+ _returnvalue (* (`self.GetActorForwardVector` (`GameplayStatics.GetPlayerCameraManager` 0)) (`self.Hook Distance`))) 5.0 "TraceTypeQuery1"))
    (if _returnvalue_2
      (set `self.Hook Point` (`.ImpactPoint` (`GameplayStatics.BreakHitResult` _outhit)))
      (set `self.Grapple Connected` true)
      (`self.SpawnGrapple`)))
  (:`Released`
    (set `self.isRightDown` false)
    (set `self.Grapple Connected` false)
    (`SceneComponent.SetHiddenInGame` (`self.Cable`) true false)))

(event `self.ReceiveDestroyed`
  ;[1 1 1] Respawn player
  (if (`self.Grapple Connected`)
    (set `self.Grapple Connected` false)
    (`SceneComponent.SetHiddenInGame` (`self.Cable`) true false))
  (`KismetSystemLibrary.Delay` 5.0)
  (`GameplayStatics.OpenLevel` (`self.Level Name`)))

(fn `SpawnBullet`
  (bind _returnvalue (`SceneComponent.K2_GetComponentRotation` (`self.Camera`)))
  (`|SpawnActorFromClass` "/Game/GrapplingHookGame/Player/Blueprints/BulletBP.BulletBP_C" (`KismetMathLibrary.MakeTransform` (+ (`SceneComponent.K2_GetComponentLocation` (`self.GunMark`)) (`KismetMathLibrary.GreaterGreater_VectorRotator` (`self.Gun offset`) _returnvalue)) _returnvalue) "AdjustIfPossibleButDontSpawnIfColliding" "OverrideRootScale" null null))

(fn `SpawnGrapple`
  (`SceneComponent.SetHiddenInGame` (`self.Cable`) false false)
  (bind _returnvalue (`|SpawnActorFromClass` "/Game/GrapplingHookGame/Player/Blueprints/HookPoint.HookPoint_C" (`KismetMathLibrary.MakeTransform` (`self.Hook Point`)) "Undefined" "OverrideRootScale" null null))
  (bind _output_get (set `self.Hook Point Actor` _returnvalue))
  (`CableComponent.SetAttachEndTo` (`self.Cable`) _output_get "None" "None"))

(fn `UserConstructionScript`)